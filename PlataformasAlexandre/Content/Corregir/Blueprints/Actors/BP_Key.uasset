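; BP_Key is a collectible key actor that feeds a puzzle Blueprint when the player picks it up.
; On BeginPlay it stores its starting transform.
; When the third-person character overlaps its sphere, it reports its KeyID to BPPuzzle, then hides itself and disables collision instead of being destroyed.
; ResetKey teleports it back to the stored transform and restores visibility and collision.
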(event `ResetKey`
  ;[1 1 1] Al resetear la llave se le devuelven sus propiedades visuales y colision y se la vuelve a colocar donde pertenece
  (`self.K2_SetActorTransform` (stale `self.ReceiveBeginPlay` _output_get) false true)
  (`self.SetActorHiddenInGame` false)
  (`self.SetActorEnableCollision` true))

(event `self.ReceiveBeginPlay`
  ;[1 1 1] Al empezar la partida se guarda la posicion actual
  (bind _output_get (set `self.InitialTransform` (`self.GetTransform`))))

(event `self.Sphere.OnComponentBeginOverlap`
  (params (OverlappedComponent :type "PrimitiveComponent Object Reference") (OtherActor :type "Actor Object Reference") (OtherComp :type "PrimitiveComponent Object Reference") (OtherBodyIndex :type Integer) (bFromSweep :type Boolean) (SweepResult :type "HitResult Structure (by ref)"))
  ;[1 1 1] Al recoger una llave se llama al Key Picked y despues se le quitan sus propiedades a la llave para hacera desaparecer
  (cast `/Game/Corregir/Blueprints/Actors/BP_ThirdPersonCharacter` OtherActor)
  (`/Game/Corregir/Blueprints/Characters/BP_PuzzleKeys.OnKeyPicked` (`self.BP_Puzzle`) (`self.KeyID`))
  (`self.SetActorHiddenInGame` true)
  (`self.SetActorEnableCollision` false))

(fn `UserConstructionScript`)