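; BP_GameManager holds the player's checkpoint and power-up state and handles respawning.
; SetCheckpoint stores a transform, which RespawnPlayer uses to teleport the BP_ThirdPersonCharacter pawn back.
; GrantPowerUp switches on a power-up enum: Running Boots sets a flag and raises walk speed, while Jetpack only sets its flag.
; Each action prints a debug message, and the event graph has no active logic.
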(fn `GrantPowerUp`
  (params (PowerUpTyper :type "/Game/Corregir/Blueprints/Actors/EPowerType Enum" :default "NewEnumerator0"))
  ;[1 1 1] Con el enumerador comprovamos con que se ha colisionado y le asignamos ese Power UP
  (switch `/Game/Corregir/Blueprints/Actors/EPowerType` PowerUpTyper
    (:`NewEnumerator0`
      (set `self.bHasSprintBoots` true)
      (bind _asbp_third_person_character (cast `/Game/Corregir/Blueprints/Actors/BP_ThirdPersonCharacter` (`GameplayStatics.GetPlayerPawn` 0)))
      (set `CharacterMovementComponent.MaxWalkSpeed` 1200.0 (`Character.CharacterMovement` _asbp_third_person_character))
      (`KismetSystemLibrary.PrintString` "Sprint Activado")
      (return))
    (:`NewEnumerator1`
      (set `self.bHasJetpack` true)
      (`KismetSystemLibrary.PrintString` "Jetpack ONLINE")
      (return))))

(fn `RespawnPlayer`
  (bind _asbp_third_person_character (cast `/Game/Corregir/Blueprints/Actors/BP_ThirdPersonCharacter` (`GameplayStatics.GetPlayerPawn` 0)))
  (`self.K2_SetActorTransform` _asbp_third_person_character (`self.Checkpoint`) false true)
  (`KismetSystemLibrary.PrintString` "Respawneando")
  (return))

(fn `SetCheckpoint`
  (params (NewCheckpoint :type "Transform Structure"))
  (set `self.Checkpoint` NewCheckpoint)
  (`KismetSystemLibrary.PrintString` "Checkpoint Seteado")
  (return))

(fn `UserConstructionScript`)