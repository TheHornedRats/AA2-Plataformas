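; BP_PuzzleKeys runs a timed two-key puzzle that opens a door.
; OnKeyPicked flags the key by ID, then either opens PuertaRef and stops the timer or starts a looping one-second countdown.
; Each tick decrements CountDownTime itself, printing it and playing audio; CurrentTime only holds the starting value.
; At zero, ResetPuzzle clears both flags, restores a hard-coded ten-second count and resets the key actors.
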(event `OnKeyPicked`
  (params (KeyId :type Integer64))
  ;[1 1 1] Al recoger una llave se comprueva su ID para marcar que se tiene
  (switch `int` (`KismetMathLibrary.Conv_Int64ToInt` KeyId)
    (:`0`
      (set `self.HasKey1` true))
    (:`1`
      (set `self.HasKey2` true)))
  (`|ExecutionSequence`
    (:`then_1`
      ;[1 1 1] Después se comprueva si se tienen las dos, en caso afirmativo se abre la puerta y se le indica al jugador
      (if (and (`self.HasKey1`) (`self.HasKey2`))
        (`KismetSystemLibrary.K2_ClearAndInvalidateTimerHandle` (`self.TimeHandle_Countdown`))
        (`/Game/Corregir/Blueprints/Actors/BP_DoorPuzzle.OpenDoor` (`self.PuertaRef`))
        (`KismetSystemLibrary.PrintString` "Puerta abierta")
        (else
          (`self.StartCountdown`))))))

(fn `ResetPuzzle`
  (bind _key1ref (`self.Key1Ref`))
  ;[1 1 1] SI el contador se termina se le quitan las llaves al jugador, se vuelven a colocar y se para el timer
  (set `self.HasKey1` false)
  (set `self.HasKey2` false)
  (set `self.CountDownTime` 10)
  (`KismetSystemLibrary.K2_ClearAndInvalidateTimerHandle` (`self.TimeHandle_Countdown`))
  (if (`KismetSystemLibrary.IsValid` _key1ref)
    (`/Game/Corregir/Blueprints/Actors/BP_Key.ResetKey` _key1ref)
    (if (`KismetSystemLibrary.IsValid` (`self.Key2Ref`))
      (`/Game/Corregir/Blueprints/Actors/BP_Key.ResetKey` (`self.Key2Ref`)))))

(fn `StartCountdown`
  ;[1 1 1] El countdown
  (set `self.CurrentTime` (`self.CountDownTime`))
  (bind _returnvalue (`KismetSystemLibrary.K2_SetTimer` null "TickCountdown" 1.0 true))
  (set `self.TimeHandle_Countdown` _returnvalue)
  (`KismetSystemLibrary.PrintString` (`KismetStringLibrary.Conv_Int64ToString` (`self.CurrentTime`))))

(fn `TickCountdown`
  ;[1 1 1] En cada tick se comprueva si se ha terminado el tiempo o si se tienen las dos llaves, para volver a reiniciar el puzzle
  (if (> (`self.CountDownTime`) 0)
    (bind _output_get (set `self.CountDownTime` (- (`self.CountDownTime`) 1)))
    (`KismetSystemLibrary.PrintString` (`KismetStringLibrary.Conv_Int64ToString` _output_get))
    (`AudioComponent.Play` (`self.Audio`) 0.0)
    (if (and (== (and (`self.HasKey1`) (`self.HasKey2`)) false) (== (`self.CurrentTime`) 0))
      _)
    (else
      (`KismetSystemLibrary.K2_ClearAndInvalidateTimerHandle` (`self.TimeHandle_Countdown`))
      (`self.ResetPuzzle`)
      (`KismetSystemLibrary.PrintString` "No conseguiste la segunda llave a timepo"))))

(fn `UserConstructionScript`)